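; BP_Dialogue is a Blueprint that shows a sequence of dialogue lines on screen, one per call to Talk.
; Each call increments an index, removes any existing WB_Dialogue widgets, and creates a new one displaying the matching DialogueText entry.
; Past the last line, it resets the index to -1 and leaves the dialogue widget cleared, so the next call restarts the conversation.
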(event EventBeginPlay)

(event EventTick
  (params (DeltaSeconds :type Float%20%28single-precision%29)))

(fn Talk
  (Variables|Default|Setindex (+ (Variables|Default|Getindex) 1))
  (bind _foundwidgets (Widget|GetAllWidgetsOfClass "/Game/MyContent/DialogueSystem/WB_Dialogue.WB_Dialogue_C" true))
  (for _array_element _foundwidgets
    (Widget|RemovefromParent _array_element))
  (bind _returnvalue (UserInterface|CreateWidget "/Game/MyContent/DialogueSystem/WB_Dialogue.WB_Dialogue_C"))
  (if (< (Variables|Default|Getindex) (Utilities|Array|Length (Variables|Default|GetDialogueText)))
    (Rendering|Components|TextRender|SetText (Variables|/Game/MyContent/DialogueSystem/WB_Dialogue.WB_Dialogue_C|GetTextBlock_0 _returnvalue) (Utilities|Text|ToText(String) (Utilities|Array|Get(acopy) (Variables|Default|GetDialogueText) (Variables|Default|Getindex))))
    (UserInterface|Viewport|AddtoViewport _returnvalue 0)
    (else
      (Variables|Default|Setindex -1)
      (bind _foundwidgets_2 (Widget|GetAllWidgetsOfClass "/Game/MyContent/DialogueSystem/WB_Dialogue.WB_Dialogue_C" true))
      (for _array_element_2 _foundwidgets_2
        (Widget|RemovefromParent _array_element_2)))))