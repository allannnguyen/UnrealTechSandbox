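; BP_NPC is a talkable character in the dialogue system that shows a widget when the player is nearby.
; A BP_Player entering TriggerSphere reveals the widget, and the Talk event forwards to the BPDialogue component.
; Any actor leaving the sphere, with no class check, hides the widget, removes all top-level WB_Dialogue widgets and resets the dialogue index.
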(event OnComponentBeginOverlap(TriggerSphere)
  (params (OverlappedComponent :type Primitive%20Component%20Object%20Reference) (OtherActor :type Actor%20Object%20Reference) (OtherComp :type Primitive%20Component%20Object%20Reference) (OtherBodyIndex :type Integer) (bFromSweep :type Boolean) (SweepResult :type Hit%20Result%20Structure%20%28by%20ref%29))
  (if (Utilities|ClassIsChildOf (Utilities|GetClass OtherActor) "/Game/MyContent/DamageSystem/BP_Player.BP_Player_C")
    (Rendering|SetVisibility (Variables|Default|GetWidget) true false)))

(event OnComponentEndOverlap(TriggerSphere)
  (params (OverlappedComponent :type Primitive%20Component%20Object%20Reference) (OtherActor :type Actor%20Object%20Reference) (OtherComp :type Primitive%20Component%20Object%20Reference) (OtherBodyIndex :type Integer))
  (Rendering|SetVisibility (Variables|Default|GetWidget) false false)
  (bind _foundwidgets (Widget|GetAllWidgetsOfClass "/Game/MyContent/DialogueSystem/WB_Dialogue.WB_Dialogue_C" true))
  (for _array_element _foundwidgets
    (Widget|RemovefromParent _array_element))
  (Variables|/Game/MyContent/DialogueSystem/BP_Dialogue.BP_Dialogue_C|Setindex (Variables|Default|GetBP_Dialogue) -1))

(event EventTalk
  (Default|Talk (Variables|Default|GetBP_Dialogue)))

(fn ConstructionScript)