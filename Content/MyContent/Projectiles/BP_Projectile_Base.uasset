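; Base projectile actor that flies at a target, optionally homing, and deals fixed damage on impact.
; Construction applies speed and gravity; BeginPlay binds to the first BP_Player's third-person-spawned event, which sets the target and redirects velocity toward it.
; A box hit fires the impact dispatcher, which the projectile itself binds to send damage through a message, then spawns effect and sound and destroys the actor.
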(event OnComponentHit(BoxCollision)
  (params (HitComponent :type Primitive%20Component%20Object%20Reference) (OtherActor :type Actor%20Object%20Reference) (OtherComp :type Primitive%20Component%20Object%20Reference) (NormalImpulse :type Vector :default "0, 0, 0") (Hit :type Hit%20Result%20Structure%20%28by%20ref%29))
  (bind _location (Collision|BreakHitResult Hit))
  (Default|CallOnProjectileImpact OtherActor Hit)
  (Effects|SpawnEmitteratLocation (Variables|Effects|GetImpact%20Effect) _location)
  (Audio|PlaySoundatLocation (Variables|Effects|GetImpact%20Sound) _location "0, 0, 0" 1.0 1.0 0.0 0 0 0 0)
  (Actor|DestroyActor))

(event Custom|RotateToTarget
  (bind _ishoming (Variables|ProjectileSettings|GetisHoming))
  (bind _projectilemovement (Variables|Default|GetProjectileMovement))
  (Variables|/Script/Engine.MovementComponent|SetVelocity (Variables|Default|GetProjectileMovement) (* (Math|Vector|GetUnitDirection(Vector) (Transformation|GetActorLocation) (Transformation|GetActorLocation (Variables|Target|GetTarget))) (Variables|ProjectileSettings|GetSpeed)))
  (if _ishoming
    (Variables|/Script/Engine.ProjectileMovementComponent|SetbIsHomingProjectile _projectilemovement _ishoming)
    (Variables|/Script/Engine.ProjectileMovementComponent|SetHomingTargetComponent _projectilemovement (Variables|/Script/Engine.Actor|GetRootComponent (Variables|Target|GetTarget)))))

(event Custom|HandleThirdPersonSpawned
  (params (BP_ThirdPerson :type Actor%20Object%20Reference))
  (Variables|Target|SetTarget BP_ThirdPerson)
  (Variables|Target|GetTarget
    (:then
      (CallFunction|RotatetoTarget))
    (:else)))

(event Custom|OnProjectileImpact_Event
  (params (Other%20Actor :type Actor%20Object%20Reference) (Hit%20Result :type Hit%20Result%20Structure))
  (Class|BPIDamageable|TakeDamage(Message) Other%20Actor (Utilities|Struct|MakeDamageInfo 2e+01)))

(event EventBeginPlay
  (bind _outactors (Actor|GetAllActorsOfClass "/Game/MyContent/DamageSystem/BP_Player.BP_Player_C"))
  (EventDispatchers|BindEventtoOnThirdPersonSpawned (Utilities|Array|Get(acopy) _outactors) (delegate Custom|HandleThirdPersonSpawned))
  (EventDispatchers|BindEventtoOnProjectileImpact (delegate Custom|OnProjectileImpact_Event)))

(fn ConstructionScript
  (bind _projectilemovement (Variables|Default|GetProjectileMovement))
  (bind _speed (Variables|ProjectileSettings|GetSpeed))
  (Variables|/Script/Engine.ProjectileMovementComponent|SetInitialSpeed _projectilemovement _speed)
  (Variables|/Script/Engine.ProjectileMovementComponent|SetMaxSpeed _projectilemovement _speed)
  (Variables|/Script/Engine.ProjectileMovementComponent|SetProjectileGravityScale _projectilemovement (Variables|ProjectileSettings|GetGravity))
  (Variables|Target|GetTarget
    (:then)
    (:else)))