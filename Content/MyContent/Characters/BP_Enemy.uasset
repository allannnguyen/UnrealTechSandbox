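; Enemy character that can take damage and shows a health bar that turns to face the player camera each tick.
; Health queries and damage delegate to the BPDamageSystem component, while Heal is a stub returning zero.
; BeginPlay creates the health bar widget with the enemy as its damageable actor.
; Surviving hits play a hit-react montage; death sets IsDead, clears the widget and disables capsule collision.
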(event EventBeginPlay
  ;[1 1 1] Set up widgets
  (bind _returnvalue (UserInterface|CreateWidget "/Game/MyContent/UI/W_EnemyHealthBar.W_EnemyHealthBar_C" 0 self))
  (UserInterface|SetWidget (Variables|Default|GetHealth%20Bar) _returnvalue))

(event Collision|EventActorBeginOverlap
  (params (OtherActor :type Actor%20Object%20Reference)))

(event EventTick
  (params (DeltaSeconds :type Float%20%28single-precision%29))
  ;[1 1 1] Rotate healthbar to camera
  (Transformation|SetWorldRotation (Variables|Default|GetHealth%20Bar) (Math|Rotator|FindLookatRotation (Transformation|GetWorldLocation (Variables|Default|GetHealth%20Bar)) (Camera|GetCameraLocation (Game|GetPlayerCameraManager 0))) false false))

(fn ConstructionScript)

(fn GetCurrentHealth
  (bind _health (Default|GetHealth (Variables|Default|GetBP_DamageSystem)))
  (return _health))

(fn GetMaxHealth
  (return (Variables|/Game/MyContent/Gameplay/DamageSystem/BP_DamageSystem.BP_DamageSystem_C|GetmaxHealth (Variables|Default|GetBP_DamageSystem))))

(fn Heal
  (params (amount :type Float%20%28double-precision%29))
  (return 0.0))

(fn TakeDamage
  (params (DamageInfo :type Damage%20Info%20Structure))
  (bind _tookdamage (Default|TakeDamage (Variables|Default|GetBP_DamageSystem) DamageInfo))
  (bind _currenthealth (CallFunction|GetCurrentHealth))
  (if (<= _currenthealth 0.0)
    (Variables|Default|SetisDead true)
    (UserInterface|SetWidget (Variables|Default|GetHealth%20Bar) 0)
    (Collision|SetCollisionEnabled (Variables|Collision|GetCapsuleComponent) "NoCollision")
    (else
      (Animation|PlayAnimMontage "/Game/MyContent/Characters/NPC/Animations/Hit_React_1_Montage.Hit_React_1_Montage" 1.0 "None")))
  (return _tookdamage))