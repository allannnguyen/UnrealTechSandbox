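; BP_DamageSystem is a basic health and damage Blueprint that tracks Health, MaxHealth and a death flag.
; TakeDamage subtracts the damage amount from a DamageInfo input, sets IsDead at zero health and always returns true.
; Heal adds health without clearing or checking IsDead, and both functions clamp Health between zero and MaxHealth.
; Getters expose current and maximum health, and the event graph has no active logic.
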(event EventBeginPlay)

(event EventTick
  (params (DeltaSeconds :type Float%20%28single-precision%29)))

(fn Heal
  (params (healAmount :type Float%20%28double-precision%29))
  (bind _output_get (Variables|Default|Sethealth (Math|Float|Clamp(Float) (+ (Variables|Default|Gethealth) healAmount) 0.0 (Variables|Default|GetmaxHealth))))
  (return _output_get))

(fn TakeDamage
  (params (Damage%20Info :type Damage%20Info%20Structure))
  (bind _output_get (Variables|Default|Sethealth (Math|Float|Clamp(Float) (- (Variables|Default|Gethealth) (Utilities|Struct|BreakDamageInfo Damage%20Info)) 0.0 (Variables|Default|GetmaxHealth))))
  (if (<= _output_get 0.0)
    (Variables|Default|SetisDead true))
  (return true))

(fn GetHealth
  (return (Variables|Default|Gethealth)))

(fn GetMaxHealth
  (return (Variables|Default|GetmaxHealth)))